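; Checkpoint actor for a vehicle race that advances the BP_ZoomyZoomPawn's checkpoint counter when it passes through.
; On leaving the Box, the pawn's velocity is dotted with the Arrow's forward vector so only forward crossings count.
; A valid crossing hides the particle marker, disables the Box and increments the pawn's CurrentCheckpoint.
; Box collision also starts disabled at BeginPlay, and nothing in this Blueprint re-enables it.
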(event OnComponentEndOverlap(Box)
  (params (OverlappedComponent :type Primitive%20Component%20Object%20Reference) (OtherActor :type Actor%20Object%20Reference) (OtherComp :type Primitive%20Component%20Object%20Reference) (OtherBodyIndex :type Integer))
  (bind _asbp_zoomy_zoom_pawn (Utilities|Casting|CastToBP_ZoomyZoomPawn OtherActor))
  (bind _output_get (Variables|Default|SetVehicle%20Reference%202 _asbp_zoomy_zoom_pawn))
  (if (> (Math|Vector|DotProduct (Transformation|GetVelocity _output_get) (Math|Rotator|GetRotationXVector (Transformation|GetWorldRotation (Variables|Default|GetArrow)))) 0.0)
    (Development|SetHiddeninGame (Variables|Default|GetParticleSystem) true false)
    (Collision|SetCollisionEnabled (Variables|Default|GetBox) "NoCollision")
    (Variables|/Game/Blueprints/BP_ZoomyZoomPawn.BP_ZoomyZoomPawn_C|SetCurrentCheckpoint (Variables|Default|GetVehicle%20Reference%202) (+ (Variables|/Game/Blueprints/BP_ZoomyZoomPawn.BP_ZoomyZoomPawn_C|GetCurrentCheckpoint (Variables|Default|GetVehicle%20Reference%202)) 1))))

(event EventBeginPlay
  (Collision|SetCollisionEnabled (Variables|Default|GetBox) "NoCollision"))

(event Collision|EventActorBeginOverlap
  (params (OtherActor :type Actor%20Object%20Reference)))

(event EventTick
  (params (DeltaSeconds :type Float%20%28single-precision%29)))

(fn ConstructionScript)