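; Checkpoint tracker that follows the player's BP_ZoomyZoomPawn progress through an array of checkpoints.
; BeginPlay caches the pawn, then reveals the particle effect and enables box collision on its current checkpoint.
; Tick repeats that activation by polling CurrentCheckpoint, and sets the pawn's RespawnLocation to the previous checkpoint's location once past the first.
; It only reads the index and never deactivates checkpoints itself.
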(event EventBeginPlay
  (bind _asbp_zoomy_zoom_pawn (Utilities|Casting|CastToBP_ZoomyZoomPawn (Game|Player|GetPlayerPawn 0)))
  (Variables|Default|SetVehicle%20Reference%202 _asbp_zoomy_zoom_pawn)
  (Development|SetHiddeninGame (Variables|/Game/Blueprints/Checkpoint.Checkpoint_C|GetParticleSystem (Utilities|Array|Get(acopy) (Variables|Default|GetCheckpoints) (Variables|/Game/Blueprints/BP_ZoomyZoomPawn.BP_ZoomyZoomPawn_C|GetCurrentCheckpoint (Variables|Default|GetVehicle%20Reference%202)))) false false)
  (Collision|SetCollisionEnabled (Variables|/Game/Blueprints/Checkpoint.Checkpoint_C|GetBox (Utilities|Array|Get(acopy) (Variables|Default|GetCheckpoints) (Variables|/Game/Blueprints/BP_ZoomyZoomPawn.BP_ZoomyZoomPawn_C|GetCurrentCheckpoint (Variables|Default|GetVehicle%20Reference%202)))) "QueryAndPhysics"))

(event Collision|EventActorBeginOverlap
  (params (OtherActor :type Actor%20Object%20Reference)))

(event EventTick
  (params (DeltaSeconds :type Float%20%28single-precision%29))
  (bind _checkpoints (Variables|Default|GetCheckpoints))
  (bind _vehicle_reference_2 (Variables|Default|GetVehicle%20Reference%202))
  (bind _currentcheckpoint (Variables|/Game/Blueprints/BP_ZoomyZoomPawn.BP_ZoomyZoomPawn_C|GetCurrentCheckpoint _vehicle_reference_2))
  (bind _output (Utilities|Array|Get(acopy) _checkpoints _currentcheckpoint))
  (Development|SetHiddeninGame (Variables|/Game/Blueprints/Checkpoint.Checkpoint_C|GetParticleSystem _output) false false)
  (Collision|SetCollisionEnabled (Variables|/Game/Blueprints/Checkpoint.Checkpoint_C|GetBox _output) "QueryAndPhysics")
  (if (> (Variables|/Game/Blueprints/BP_ZoomyZoomPawn.BP_ZoomyZoomPawn_C|GetCurrentCheckpoint (Variables|Default|GetVehicle%20Reference%202)) 0)
    (Variables|/Game/Blueprints/BP_ZoomyZoomPawn.BP_ZoomyZoomPawn_C|SetRespawnLocation (Variables|Default|GetVehicle%20Reference%202) (Transformation|GetActorLocation (Utilities|Array|Get(acopy) (Variables|Default|GetCheckpoints) (- (Variables|/Game/Blueprints/BP_ZoomyZoomPawn.BP_ZoomyZoomPawn_C|GetCurrentCheckpoint (Variables|Default|GetVehicle%20Reference%202)) 1))))))

(fn ConstructionScript)